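; Blueprint function library for on-screen debug logging at Debug, Info, Warning and Error levels.
; LogDebug, LogInfo, LogWarning and LogError each forward a message and caller to a shared Log function with their level.
; Log prints a string prefixed with the level and caller name, colored by severity, using the caller as world context.
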(fn `Log`
  (params (message :type String) (Caller :type "Object Object Reference") (Level :type "/Game/BluePrints/LogLevels Enum" :default "NewEnumerator0"))
  (`KismetSystemLibrary.PrintString` Caller (`KismetStringLibrary.Concat_StrStr` "[" (`|GetEnumeratorNameAsString` Level) "]" "[" (`VictoryBPFunctionLibrary.Accessor__GetNameAsString` Caller) "]:" message) true true (select `/Game/BluePrints/LogLevels` Level :`NewEnumerator0` (struct :`R` 0.991102 :`G` 0.90232 :`A` 1.0) :`NewEnumerator1` (struct :`R` 1.0 :`G` 1.0 :`B` 1.0 :`A` 1.0) :`NewEnumerator2` (struct :`R` 0.991102 :`G` 0.584079 :`B` 0.051269 :`A` 1.0) :`NewEnumerator3` (struct :`R` 1.0 :`A` 1.0) :!type "LinearColor Structure") 5.0))

(fn `LogDebug`
  (params (Message :type String) (Caller :type "Object Object Reference"))
  (`self.Log` Message Caller "NewEnumerator0"))

(fn `LogError`
  (params (message :type String) (Caller :type "Object Object Reference"))
  (`self.Log` message Caller "NewEnumerator3"))

(fn `LogInfo`
  (params (message :type String) (Caller :type "Object Object Reference"))
  (`self.Log` message Caller "NewEnumerator1"))

(fn `LogWarning`
  (params (Message :type String) (Caller :type "Object Object Reference"))
  (`self.Log` Message Caller "NewEnumerator2"))