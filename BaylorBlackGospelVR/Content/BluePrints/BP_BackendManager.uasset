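; Backend manager that pulls record metadata from the CONTENTdm fa-gospel collection, then registers itself with Spawner and calls SpawnInitialRecords.
; Event-graph HTTP requests query record IDs, then each record's item info and file structure.
; Parse functions read the XML into RecordMetaData: artist, year, titles, image and song pointers, stripping the UTF-8 BOM from the structure response.
; An image download chain exists but is never run.
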(event `self.ReceiveBeginPlay`
  (bind _spawner (`self.Spawner`))
  ;[1 1 1] Construct the set of records at the start
  (`self.FetchRecordPointers`)
  (set `/Game/BluePrints/BP_ItemSpawner.BackendManager` self _spawner)
  (`/Game/BluePrints/BP_ItemSpawner.SpawnInitialRecords` _spawner))

(event `FetchRecordPointers`
  ;[1 1 1] Fetch the initial record pointers (record IDs)
  (bind _returnvalue (`LowEntryHttpRequestLibrary.Request_Create`))
  (`LowEntryHttpRequest.SetUrl` _returnvalue "GET" "https://server17178.contentdm.oclc.org/dmwebservices/index.php?q=dmQuery/fa-gospel/CISOSEARCHALL/title/title/1/3/xml")
  (bind _response (`LowEntryHttpRequest.ExecuteRequest` _returnvalue)) ; Can only be executed within the event graph (NOT in a function)
  (`self.ParseRecordPointers` _response)
  (`self.FetchRecordMetaData`))

(event `FetchRecordMetaData`
  ;[1 1 1] Fetch each record's metadata
  (for (_array_element _array_index) (`self.RecordMetaData`)
    (bind _returnvalue (`LowEntryHttpRequestLibrary.Request_Create`))
    (`LowEntryHttpRequest.SetUrl` _returnvalue "GET" (`KismetStringLibrary.Concat_StrStr` "https://server17178.contentdm.oclc.org/dmwebservices/index.php?q=dmGetItemInfo/fa-gospel/" (`KismetStringLibrary.Conv_IntToString` (break `/Game/BluePrints/RecordMetaData` _array_element)) "/xml"))
    (bind _response (`LowEntryHttpRequest.ExecuteRequest` _returnvalue)) ; Can only be executed within the event graph (NOT in a function)
    (`self.ParseRecordMetaData` _response _array_index)
    (bind _returnvalue_2 (`LowEntryHttpRequestLibrary.Request_Create`))
    (`LowEntryHttpRequest.SetUrl` _returnvalue_2 "GET" (`KismetStringLibrary.Concat_StrStr` "https://server17178.contentdm.oclc.org/dmwebservices/index.php?q=dmGetStreamingFile/fa-gospel/" (`.MetaDataSongImage_20_EFE815D1410DD6C5A150DABB2519508D` (break `/Game/BluePrints/RecordMetaData` _array_element)) "/xml"))
    (bind _response_2 (`LowEntryHttpRequest.ExecuteRequest` _returnvalue_2)) ; Can only be executed within the event graph (NOT in a function)
    (`self.ParseImageSongMetaData` _response_2 _array_index))
  (`KismetSystemLibrary.PrintString` "Complete" true true (struct :`G` 0.66 :`B` 1.0 :`A` 1.0) 10.0))

(fn `ParseImageSongMetaData`
  (params (Response :type "LowEntryHttpRequestResponse Object Reference") (MetaDataIndex :type Integer))
  (locals (CurrentNodeTitle :type String) (`temp str` :type String))
  (bind (_output_recordpointer _output_metadatasongimage _output_artist _output_year _output_imagepointer _output_songpointer _output_titles) (break `/Game/BluePrints/RecordMetaData` (`|GetArrayItem` (`self.RecordMetaData`) MetaDataIndex)))
  (bind _returnvalue (`LowEntryXmlParserLibrary.StringToXml` (`LowEntryExtendedStandardLibrary.BytesToStringUtf8` (`LowEntryExtendedStandardLibrary.BytesSubArray` (`LowEntryHttpRequestResponse.GetContent` Response) 3)))) ; Get the XML string
  (bind _returnvalue_2 (`LowEntryXmlParserNode.FindChildNode` _returnvalue "node")) ; Find the container node
  (bind _returnvalue_3 (`LowEntryXmlParserNode.GetChildrenNodes` _returnvalue_2))
  (for _array_element _returnvalue_3
    (if (`KismetStringLibrary.EqualEqual_StrStr` (`LowEntryXmlParserNode.GetTag` _array_element) "node")
      (bind _returnvalue_4 (`LowEntryXmlParserNode.GetChildrenNodes` _array_element)) ; Get that nodes children
      (for _array_element_2 _returnvalue_4
        (if (`KismetStringLibrary.EqualEqual_StrStr` (`LowEntryXmlParserNode.GetTag` _array_element_2) "nodetitle")
          (set `local.CurrentNodeTitle` (`LowEntryXmlParserNode.GetValue` _array_element_2))
          (elif (`KismetStringLibrary.EqualEqual_StrStr` (`LowEntryXmlParserNode.GetTag` _array_element_2) "page")
            (if (`KismetStringLibrary.Contains` (`local.CurrentNodeTitle`) "images")
              (bind _returnvalue_5 (`LowEntryXmlParserNode.FindChildNode` _array_element_2 "pageptr"))
              (`/Engine/EditorBlueprintResources/StandardMacros.IsValid` _returnvalue_5
                (:`Is Valid`
                  (`KismetArrayLibrary.Array_Add` _output_imagepointer (`LowEntryXmlParserNode.GetValue` _returnvalue_5)))
                (:`Is Not Valid`
                  (`KismetSystemLibrary.PrintString` "pagefile tag not found under node" true true (struct :`R` 1.0 :`A` 1.0) 5.0 :!label _label)))
              (elif (`KismetStringLibrary.Contains` (`local.CurrentNodeTitle`) "audio")
                (`|ExecutionSequence`
                  (:`then_0`
                    (bind _returnvalue_6 (`LowEntryXmlParserNode.FindChildNode` _array_element_2 "pagefile"))
                    (`/Engine/EditorBlueprintResources/StandardMacros.IsValid` _returnvalue_6
                      (:`Is Valid`
                        (`KismetArrayLibrary.Array_Add` _output_songpointer (`LowEntryXmlParserNode.GetValue` _returnvalue_6)))
                      (:`Is Not Valid`
                        (goto _label))))
                  (:`then_1`
                    (bind _returnvalue_7 (`LowEntryXmlParserNode.FindChildNode` _array_element_2 "pagetitle"))
                    (`/Engine/EditorBlueprintResources/StandardMacros.IsValid` _returnvalue_7
                      (:`Is Valid`
                        (`KismetArrayLibrary.Array_Add` _output_titles (`LowEntryXmlParserNode.GetValue` _returnvalue_7))))))
                (else
                  (`KismetSystemLibrary.PrintString` "ERROR: did not find images or audio nodetitle!" true true (struct :`R` 1.0 :`A` 1.0) 5.0)))))))))
  (`KismetSystemLibrary.PrintString` "Hello"))

(fn `ParseRecordMetaData`
  (params (Response :type "LowEntryHttpRequestResponse Object Reference") (MetaDataIndex :type Integer))
  (bind (_output_recordpointer _output_metadatasongimage _output_artist _output_year) (break `/Game/BluePrints/RecordMetaData` (`|GetArrayItem` (`self.RecordMetaData`) MetaDataIndex)))
  (bind _returnvalue (`LowEntryXmlParserLibrary.StringToXml` (`LowEntryHttpRequestResponse.GetContentAsString` Response)))
  (`|ExecutionSequence`
    (:`then_0`
      (bind _returnvalue_2 (`LowEntryXmlParserNode.FindChildNode` _returnvalue "find")) ; Get the record's song data pointer
      (`|VariableSetRef` _output_metadatasongimage (`LowEntryXmlParserNode.GetValue` _returnvalue_2)))
    (:`then_1`
      (bind _returnvalue_3 (`LowEntryXmlParserNode.FindChildNode` _returnvalue "artist")) ; Get the record's artist
      (`|VariableSetRef` _output_artist (`LowEntryXmlParserNode.GetValue` _returnvalue_3)))
    (:`then_2`
      (bind _returnvalue_4 (`LowEntryXmlParserNode.FindChildNode` _returnvalue "origic")) ; Get the record's publication date
      (`|VariableSetRef` _output_year (`LowEntryXmlParserNode.GetValue` _returnvalue_4)))))

(fn `ParseRecordPointers`
  (params (Response :type "LowEntryHttpRequestResponse Object Reference"))
  (bind _returnvalue (`LowEntryXmlParserLibrary.StringToXml` (`LowEntryHttpRequestResponse.GetContentAsString` Response)))
  (bind _returnvalue_2 (`LowEntryXmlParserNode.FindChildNode` _returnvalue "records")) ; Under the "records" tag that lists the "record" nodes
  (bind _returnvalue_3 (`LowEntryXmlParserNode.GetChildrenNodes` _returnvalue_2))
  (for _array_element _returnvalue_3
    (bind _returnvalue_4 (`LowEntryXmlParserNode.FindChildNode` _array_element "pointer")) ; Find the ID of the "record" (called "pointer" in XML)
    (bind _returnvalue_5 (`LowEntryXmlParserNode.GetValue` _returnvalue_4))
    (`KismetArrayLibrary.Array_Add` (`self.RecordMetaData`) (make `/Game/BluePrints/RecordMetaData` (`KismetStringLibrary.Conv_StringToInt` _returnvalue_5) "-1" "" "" (`|MakeArray`) (`|MakeArray`) (`|MakeArray`)))
    (`KismetSystemLibrary.PrintString` _returnvalue_5 true true (struct :`A` 1.0) 10.0))
  (`KismetSystemLibrary.PrintString` (`KismetStringLibrary.Concat_StrStr` (`KismetStringLibrary.Conv_IntToString` (`KismetArrayLibrary.Array_Length` (`self.RecordMetaData`))) " record IDs fetched.") true true (struct :`A` 1.0) 5.0))

(fn `UserConstructionScript`)