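; BP_Record is a vinyl record actor that motion controllers can pick up and drop, toggling physics and attachment.
; FetchImage requests its disc image over HTTP from Baylor's gospel digital collection, using the first image ID in MetaData.
; ParseImage decodes the response bytes as JPEG into a Texture2D and applies it through a dynamic M_DynamicRecord material.
; It also opens the URL in a media player, though the material uses the decoded texture.
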(event `/Game/BluePrints/PickupActorInterface.Pickup`
  (params (AttachTo :type "SceneComponent Object Reference"))
  ;[1 1 1] Pick up vinyl
  (`PrimitiveComponent.SetSimulatePhysics` (`self.StaticMeshComponent`) false)
  (`SceneComponent.K2_AttachToComponent` (`self.K2_GetRootComponent`) AttachTo "None" "KeepWorld" "KeepWorld" "KeepWorld" false))

(event `/Game/BluePrints/PickupActorInterface.Drop`
  ;[1 1 1] Drop the vinyl
  (`PrimitiveComponent.SetSimulatePhysics` (`self.StaticMeshComponent`) true)
  (`self.K2_DetachFromActor` "KeepWorld" "KeepWorld" "KeepWorld"))

(fn `FetchImage`
  (bind (_metadata_recordpointer _metadata_metadatasongimage _metadata_resource _metadata_artist _metadata_year _metadata_discimages) (break `/Game/BluePrints/Structures/RecordMetaData` (`self.MetaData`)))
  (bind _returnvalue (`KismetStringLibrary.Concat_StrStr` "http://digitalcollections.baylor.edu/utils/ajaxhelper/?CISOROOT=fa-gospel&CISOPTR=" (`|GetArrayItem` _metadata_discimages) "&action=2&DMSCALE=15&DMWIDTH=500&DMHEIGHT=500&DMX=0&DMY=0&DMTEXT=&DMROTATE=0"))
  (if (!= _metadata_recordpointer -1)
    (set `StreamMediaSource.StreamUrl` _returnvalue (`self.ImageSource`))
    (bind _returnvalue_2 (`LowEntryHttpRequestLibrary.Request_Create`))
    (`LowEntryHttpRequest.SetUrl` _returnvalue_2 "GET" _returnvalue)
    (`LowEntryHttpRequest.ExecuteRequestEvent` _returnvalue_2 (`|CreateDelegate` :!event `ParseImage`))
    (else
      (`KismetSystemLibrary.PrintString` "No data in MetaData" true true (struct :`R` 1.0 :`A` 1.0) 5.0))))

(fn `ParseImage`
  (params (Response :type "LowEntryHttpRequestResponse Object Reference"))
  (bind _returnvalue (`LowEntryHttpRequestResponse.GetContent` Response))
  (bind _imageplayer (`self.ImagePlayer`))
  (`LowEntryHttpRequestResponse.WasSuccessful` Response
    (:`Success`
      (if (`KismetStringLibrary.Contains` (`LowEntryHttpRequestResponse.GetUrl` Response) "19697")
        (`KismetSystemLibrary.PrintString` "Hello"))
      (for (_ _array_index) _returnvalue
        (if (`LowEntryExtendedStandardLibrary.AreBytesEqual` _returnvalue (`LowEntryExtendedStandardLibrary.HexToBytes` "FFD8FF") 0 3 0 3)
          (break)))
      (bind (_reusedgiventexture2d _returnvalue_2) (`LowEntryExtendedStandardLibrary.BytesToExistingImage` (`self.ImageTexture2D`) (`LowEntryExtendedStandardLibrary.BytesSubArray` _returnvalue _array_index) "JPEG"))
      (set `self.ImageTexture2D` _returnvalue_2)
      (set `MediaPlayer.PlayOnOpen` true _imageplayer)
      (`MediaTexture.SetMediaPlayer` (`self.ImageTexture`) _imageplayer)
      (bind _returnvalue_3 (`PrimitiveComponent.CreateDynamicMaterialInstance` (`self.StaticMeshComponent`) 0 "/Game/MusicAssets/M_DynamicRecord.M_DynamicRecord" "None"))
      (`MaterialInstanceDynamic.SetTextureParameterValue` _returnvalue_3 "Texture" (`self.ImageTexture2D`))
      (`MediaPlayer.OpenSource` _imageplayer (`self.ImageSource`)))
    (:`Failed`
      (`KismetSystemLibrary.PrintString` "Request fetching record image failed" true true (struct :`R` 1.0 :`A` 1.0) 5.0))))

(fn `UserConstructionScript`
  (`|ExecutionSequence`
    (:`then_0`
      (bind _returnvalue (`|GenericCreateObject` "/Script/Engine.Texture2D" self))
      (set `self.ImageTexture2D` _returnvalue))
    (:`then_1`
      (bind _returnvalue_2 (`|GenericCreateObject` "/Script/MediaAssets.StreamMediaSource" self))
      (set `self.ImageSource` _returnvalue_2))
    (:`then_2`
      (bind _returnvalue_3 (`|GenericCreateObject` "/Script/MediaAssets.MediaTexture" self))
      (set `self.ImageTexture` _returnvalue_3))
    (:`then_3`
      (bind _returnvalue_4 (`|GenericCreateObject` "/Script/MediaAssets.MediaPlayer" self))
      (set `self.ImagePlayer` _returnvalue_4))))