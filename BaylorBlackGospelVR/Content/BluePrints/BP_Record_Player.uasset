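; Record player actor that plays a vinyl's music when a BP_Vinyl hits it, replacing any playing song.
; The track spawns as attached audio on the mesh and is remembered for replay.
; Play, Pause and Stop functions track elapsed time for resuming, though this graph's PlaySong call is unreachable.
; Motion controller pickup attaches the player, disables physics and stops the song; dropping detaches it and restores physics.
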(event `self.ReceiveHit`
  (params (MyComp :type "PrimitiveComponent Object Reference") (Other :type "Actor Object Reference") (OtherComp :type "PrimitiveComponent Object Reference") (bSelfMoved :type Boolean) (HitLocation :type "Vector Structure") (HitNormal :type "Vector Structure") (NormalImpulse :type "Vector Structure") (Hit :type "HitResult Structure (by ref)"))
  (if (`KismetMathLibrary.ClassIsChildOf` (`GameplayStatics.GetObjectClass` Other) "/Game/BluePrints/BP_Vinyl.BP_Vinyl_C")
    (if (`AudioComponent.IsPlaying` (`self.CurrentSong`))
      (`self.Stop Song`))
    (bind _asbp_vinyl (cast `/Game/BluePrints/BP_Vinyl` Other) ; Get the object as vinyl
      (:`then`
        (bind _music (`/Game/BluePrints/BP_Vinyl.Music` _asbp_vinyl))
        (set `self.last_song_played` _music)
        (bind _returnvalue (`GameplayStatics.SpawnSoundAttached` _music (`self.StaticMeshComponent`)))
        (set `self.CurrentSong` _returnvalue) ; Set the current song for the record player from the vinyl
        (set `self.ElapsedTime` 0.0))
      (:`CastFailed`
        (`KismetSystemLibrary.PrintString` "!!! ERROR: Cast failed to BP_Vinyl (after confirmation of being BP_Vinyl Instance): BP_Record_Player > Event Graph > Event Hit " true true (struct :`G` 0.66 :`B` 1.0 :`A` 1.0) 7.0)))))

(event `/Game/BluePrints/PickupActorInterface.Pickup`
  (params (AttachTo :type "SceneComponent Object Reference"))
  ;[1 1 1] When the object is picked up
  (`PrimitiveComponent.SetSimulatePhysics` (`self.StaticMeshComponent`) false)
  (`SceneComponent.K2_AttachToComponent` (`self.K2_GetRootComponent`) AttachTo "None" "KeepWorld" "KeepWorld" "KeepWorld" false)
  (`self.Stop Song`))

(event `/Game/BluePrints/PickupActorInterface.Drop`
  ;[1 1 1] Whjen the object is dropped
  (`PrimitiveComponent.SetSimulatePhysics` (`self.StaticMeshComponent`) true)
  (`self.K2_DetachFromActor` "KeepWorld" "KeepWorld" "KeepWorld"))

(fn `Pause Song`
  (`/Engine/EditorBlueprintResources/StandardMacros.IsValid` (`self.CurrentSong`) ; Verify the current song is valid
    (:`Is Valid`
      (set `self.ElapsedTime` (+ (- (`self.GetGameTimeSinceCreation`) (`self.StartTime`)) (`self.ElapsedTime`))) ; Set the new elpased time
      (`AudioComponent.Stop` (`self.CurrentSong`)) ; Pause the current playing song
    )))

(fn `Play Song`
  (bind _last_song_played (`self.last_song_played`))
  (if (`AudioComponent.IsPlaying` (`self.CurrentSong`))
    (`self.Stop Song`))
  (`SceneComponent.K2_SetWorldLocation` (`self.CurrentSong`) (`SceneComponent.K2_GetComponentLocation` (`self.StaticMeshComponent`)) false false) ; Set the song to play at the location of the record player
  (`/Engine/EditorBlueprintResources/StandardMacros.IsValid` _last_song_played
    (:`Is Valid`
      (bind _returnvalue (`GameplayStatics.SpawnSoundAttached` _last_song_played (`self.StaticMeshComponent`) "None" (0.0 0.0 0.0) (struct) "KeepRelativeOffset" true 1.0 1.0 (`self.ElapsedTime`)))
      (set `self.CurrentSong` _returnvalue) ; Set the current song for the record player from the vinyl
      (set `self.StartTime` (`KismetSystemLibrary.GetGameTimeInSeconds`)) ; Set the start time of playing this song
    )
    (:`Is Not Valid`
      (`AudioComponent.Play` (`self.CurrentSong`) (`self.ElapsedTime`)) ; Play the current song with the current elapsed time (starts at 0)
      (set `self.StartTime` (`KismetSystemLibrary.GetGameTimeInSeconds`)) ; Set the start time of playing this song
    )))

(fn `Stop Song`
  (`/Engine/EditorBlueprintResources/StandardMacros.IsValid` (`self.CurrentSong`) ; Verify the current song is valid
    (:`Is Valid`
      (`AudioComponent.Stop` (`self.CurrentSong`)) ; Stop the current playing song
      (set `self.ElapsedTime` 0.0) ; Reset the elapsed time because the song was stopped
      (set `self.CurrentSong` null) ; Clear the current song that is playing
    )))

(fn `UserConstructionScript`)