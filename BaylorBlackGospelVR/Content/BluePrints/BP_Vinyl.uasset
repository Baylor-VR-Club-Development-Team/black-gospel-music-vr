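; BP_Vinyl is a vinyl record that BP_MotionController picks up and drops by attaching or detaching it and toggling physics.
; On overlapping a BP_Record_Player it attaches its mesh to the player's mesh, then immediately destroys itself.
; Setter functions assign its Music sound and label material.
; Despite the "start music" comment, no sound plays here: BeginPlay adds an audio component, but the playback nodes are unconnected.
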(event `self.ReceiveBeginPlay`
  (`AddComponent|NODE_AddAudioComponent-1`))

(event `self.StaticMeshComponent.OnComponentBeginOverlap`
  (params (OverlappedComponent :type "PrimitiveComponent Object Reference") (OtherActor :type "Actor Object Reference") (OtherComp :type "PrimitiveComponent Object Reference") (OtherBodyIndex :type Integer) (bFromSweep :type Boolean) (SweepResult :type "HitResult Structure (by ref)")))

(event `self.ReceiveActorBeginOverlap`
  (params (OtherActor :type "Actor Object Reference"))
  ;[1 1 1] Begin Overlap - start music
  (if (`KismetMathLibrary.ClassIsChildOf` (`GameplayStatics.GetObjectClass` OtherActor) "/Game/BluePrints/BP_Record_Player.BP_Record_Player_C")
    (bind _asbp_record_player (cast `/Game/BluePrints/BP_Record_Player` OtherActor))
    (bind _staticmeshcomponent (`StaticMeshActor.StaticMeshComponent` _asbp_record_player))
    (`SceneComponent.K2_AttachToComponent` (`self.StaticMeshComponent`) _staticmeshcomponent (`SceneComponent.GetAttachSocketName` _staticmeshcomponent) "KeepRelative" "KeepRelative" "KeepRelative" true)
    (`self.K2_DestroyActor`)
    (`ActorComponent.K2_DestroyComponent` (`self.StaticMeshComponent`))))

(event `self.ReceiveActorEndOverlap`
  (params (OtherActor :type "Actor Object Reference"))
  ;[1 1 1] Begin Overlap - start music
  (if (`KismetMathLibrary.ClassIsChildOf` (`GameplayStatics.GetObjectClass` OtherActor) "/Game/BluePrints/BP_Record_Player.BP_Record_Player_C")
    _))

(event `/Game/BluePrints/PickupActorInterface.Pickup`
  (params (AttachTo :type "SceneComponent Object Reference"))
  ;[1 1 1] Pick up vinyl
  (`PrimitiveComponent.SetSimulatePhysics` (`self.StaticMeshComponent`) false)
  (`SceneComponent.K2_AttachToComponent` (`self.K2_GetRootComponent`) AttachTo "None" "KeepWorld" "KeepWorld" "KeepWorld" false))

(event `/Game/BluePrints/PickupActorInterface.Drop`
  ;[1 1 1] Drop the vinyl
  (`PrimitiveComponent.SetSimulatePhysics` (`self.StaticMeshComponent`) true)
  (`self.K2_DetachFromActor` "KeepWorld" "KeepWorld" "KeepWorld"))

(fn `set_Music`
  (params (sound :type "SoundBase Object Reference"))
  (set `self.Music` sound))

(fn `set_Vinyl_Image`
  (params (new_material :type "Material Object Reference"))
  (`PrimitiveComponent.SetMaterial` (`self.StaticMeshComponent`) 0 new_material)
  (set `self.material` new_material))

(fn `UserConstructionScript`)