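; Physical play/pause button that controls a RecordPlayer when touched by a BP_MotionController.
; Overlap and Hit events share one check, then a FlipFlop alternates between pausing and playing the song, starting with pause.
; Each press changes the mesh's Z scale to show a pressed or raised state and plays a sound at the button.
; A CanBeClicked flag with a short Delay debounces repeated touches.
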(event `self.ReceiveActorBeginOverlap`
  (params (OtherActor :type "Actor Object Reference"))
  (bind _staticmeshcomponent (`self.StaticMeshComponent`))
  (bind _recordplayer (`self.RecordPlayer`))
  (bind _returnvalue (`SceneComponent.K2_GetComponentLocation` (`self.StaticMeshComponent`)))
  ;[1 1 1] Player press button
  (if (and (`KismetMathLibrary.ClassIsChildOf` (`GameplayStatics.GetObjectClass` OtherActor) "/Game/BluePrints/BP_MotionController.BP_MotionController_C") (`self.CanBeClicked`)) :!label _label
    (`/Engine/EditorBlueprintResources/StandardMacros.FlipFlop`
      (:`A`
        (`SceneComponent.SetWorldScale3D` _staticmeshcomponent (0.5 0.5 0.2))
        (`GameplayStatics.PlaySoundAtLocation` "/Game/double_oil_can.double_oil_can" _returnvalue)
        (`/Game/BluePrints/BP_Record_Player.Pause Song` _recordplayer))
      (:`B`
        (`SceneComponent.SetWorldScale3D` _staticmeshcomponent (0.5 0.5 0.5))
        (`GameplayStatics.PlaySoundAtLocation` "/Game/StarterContent/Audio/Explosion01.Explosion01" _returnvalue)
        (`/Game/BluePrints/BP_Record_Player.Play Song` _recordplayer)))
    (set `self.CanBeClicked` false)
    (`KismetSystemLibrary.Delay` 0.3)
    (set `self.CanBeClicked` true)))

(event `self.ReceiveHit`
  (params (MyComp :type "PrimitiveComponent Object Reference") (Other :type "Actor Object Reference") (OtherComp :type "PrimitiveComponent Object Reference") (bSelfMoved :type Boolean) (HitLocation :type "Vector Structure") (HitNormal :type "Vector Structure") (NormalImpulse :type "Vector Structure") (Hit :type "HitResult Structure (by ref)"))
  ;[1 1 1] Player press button
  (goto _label))

(fn `UserConstructionScript`)