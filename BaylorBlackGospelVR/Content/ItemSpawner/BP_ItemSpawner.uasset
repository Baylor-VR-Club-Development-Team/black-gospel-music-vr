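; Item spawner actor that creates BP_Vinyl records at its location and assigns their cover material and music.
; Motion controller overlap on its widget spawns a fixed gospel record, bypassing the CurrentItem check in the uncalled AttemptSpawn helpers.
; Mouse, trigger and grab inputs drive a WidgetInteraction left click.
; BeginPlay calls an unfinished index-based spawn that only range-checks, leaving its lookup tables unconnected and spawning nothing.
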(event `Key|RightMouseButton`
  (params (Key :type "Key Structure"))
  (bind _widgetinteraction (`self.WidgetInteraction`))
  ;[1 1 1] for activating the button
  (:`Pressed`
    (`WidgetInteractionComponent.PressPointerKey` _widgetinteraction "LeftMouseButton" :!label _label))
  (:`Released`
    (`WidgetInteractionComponent.ReleasePointerKey` _widgetinteraction "LeftMouseButton" :!label _label_2)))

(event `InputAxisKey|OculusTouch_Left_FaceButton1`
  (params (AxisValue :type "Float (single-precision)")))

(event `Key|MotionController_Right_Trigger`
  (params (Key :type "Key Structure"))
  ;[1 1 1] for activating the button
  (:`Pressed`
    (goto _label))
  (:`Released`
    (goto _label_2)))

(event `InputAxisKey|OculusTouch_Left_FaceButton2`
  (params (AxisValue :type "Float (single-precision)")))

(event `InputAction|GrabLeft`
  (params (Key :type "Key Structure"))
  ;[1 1 1] for activating the button
  (:`Pressed`
    (goto _label))
  (:`Released`
    (goto _label_2)))

(event `InputAction|GrabRight`
  (params (Key :type "Key Structure"))
  ;[1 1 1] for activating the button
  (:`Pressed`
    (goto _label))
  (:`Released`
    (goto _label_2)))

(event `self.ReceiveBeginPlay`
  ;[1 1 1] Spawn first initial vinyl
  (`self.SpawnWithSoundAndPicture_INT` (`self.Start_Game_Music_Spawn_Number`)))

(event `self.Widget.OnComponentBeginOverlap`
  (params (OverlappedComponent :type "PrimitiveComponent Object Reference") (OtherActor :type "Actor Object Reference") (OtherComp :type "PrimitiveComponent Object Reference") (OtherBodyIndex :type Integer) (bFromSweep :type Boolean) (SweepResult :type "HitResult Structure (by ref)"))
  (if (`KismetMathLibrary.ClassIsChildOf` (`GameplayStatics.GetObjectClass` OtherActor) "/Game/VirtualRealityBP/Blueprints/BP_MotionController.BP_MotionController_C")
    (`self.SpawnWithSoundAndPicture` "/Game/Dust_on_the_Bible_Mat.Dust_on_the_Bible_Mat" "/Game/Dust_on_the_Bible___Where_shall_I_be_The_Black_Gospel_Music.Dust_on_the_Bible___Where_shall_I_be_The_Black_Gospel_Music")))

(fn `AttemptSpawn`
  (`/Engine/EditorBlueprintResources/StandardMacros.IsValid` (`self.CurrentItem`)
    (:`Is Valid`
      (`KismetSystemLibrary.PrintString` "Item Already Spawned"))
    (:`Is Not Valid`
      (`self.SpawnItem`))))

(fn `AttemptSpawnWithSoundAndPicture`
  (`/Engine/EditorBlueprintResources/StandardMacros.IsValid` (`self.CurrentItem`)
    (:`Is Valid`
      (`KismetSystemLibrary.PrintString` "Item Already Spawned In The Area"))
    (:`Is Not Valid`
      (`self.SpawnWithSoundAndPicture` "/Game/Dust_on_the_Bible_Mat.Dust_on_the_Bible_Mat"))))

(fn `SpawnItem`
  (bind _returnvalue (`|SpawnActorFromClass` "/Game/VirtualRealityBP/Blueprints/BP_Vinyl.BP_Vinyl_C" (`KismetMathLibrary.MakeTransform` (`self.K2_GetActorLocation`) (`self.K2_GetActorRotation`)) "Undefined" "OverrideRootScale" null null))
  (set `self.CurrentItem` _returnvalue)
  (`KismetSystemLibrary.PrintString` "The item has spawned!" true true (struct :`G` 0.66 :`B` 1.0 :`A` 1.0) 5.0))

(fn `SpawnWithSoundAndPicture`
  (params (`New Material` :type "Material Object Reference") (`New Sound` :type "SoundWave Object Reference"))
  ;[1 1 1] Spawn vinyl given the material and the music
  (bind _returnvalue (`|SpawnActorFromClass` "/Game/VirtualRealityBP/Blueprints/BP_Vinyl.BP_Vinyl_C" (`KismetMathLibrary.MakeTransform` (`self.K2_GetActorLocation`) (`self.K2_GetActorRotation`)) "Undefined" "OverrideRootScale" null null))
  (bind _output_get (set `self.CurrentItem` _returnvalue))
  (`/Game/VirtualRealityBP/Blueprints/BP_Vinyl.set_Vinyl_Image` _output_get `New Material`)
  (`/Game/VirtualRealityBP/Blueprints/BP_Vinyl.set_Music` _output_get `New Sound`))

(fn `SpawnWithSoundAndPicture_INT`
  (params (ToFind :type Integer))
  (if (not (and (< ToFind 25) (> ToFind -1)))
    (`KismetSystemLibrary.PrintString` "Error: 1-25 for top 25 vinyl spawn is out of range ")))

(fn `UserConstructionScript`)